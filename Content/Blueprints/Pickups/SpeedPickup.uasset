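; Speed boost pickup that temporarily multiplies the walk speed of the MyCharacter that overlaps it.
; On overlap it hides the mesh, disables its hit box and briefly toggles a particle effect.
; It then raises MaxWalkSpeed by a multiplier for a set duration, restores the saved speed and destroys itself.
; The construction script applies a configurable material to the mesh.
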(event `self.HitBox.OnComponentBeginOverlap`
  (params (OtherActor :type "Actor Object Reference") (OtherComp :type "PrimitiveComponent Object Reference") (OtherBodyIndex :type Integer))
  (bind _playerchar (`self.PlayerChar`))
  (bind _particlehitbox (`self.ParticleHitBox`))
  (bind _charactermovement (`Character.CharacterMovement` _playerchar))
  (bind _returnvalue (`MovementComponent.GetMaxSpeed` (`Pawn.GetMovementComponent` _playerchar)))
  (bind _asmycharacter_c (cast `/Game/Blueprints/MyCharacter` OtherActor))
  (set `self.PlayerChar` _asmycharacter_c)
  (`ActorComponent.ToggleActive` _particlehitbox)
  (`SceneComponent.SetHiddenInGame` (`self.SpeedPickupMesh`) true false)
  (`PrimitiveComponent.SetCollisionEnabled` (`self.HitBox`) "NoCollision")
  (`KismetSystemLibrary.Delay` 0.2)
  (`ActorComponent.ToggleActive` _particlehitbox)
  (set `self.Original Speed` _returnvalue)
  (set `CharacterMovementComponent.MaxWalkSpeed` (* _returnvalue (`self.Speed Multiplier`)) _charactermovement)
  (`KismetSystemLibrary.Delay` (`self.Duration`))
  (set `CharacterMovementComponent.MaxWalkSpeed` (`self.Original Speed`) _charactermovement)
  (`self.K2_DestroyActor`))

(fn `UserConstructionScript`
  (`PrimitiveComponent.SetMaterial` (`self.SpeedPickupMesh`) 0 (`self.Material`)))