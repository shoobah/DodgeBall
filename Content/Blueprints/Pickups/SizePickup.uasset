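; Size powerup pickup that temporarily rescales the MyCharacter that overlaps it.
; On overlap it hides its mesh, disables the hit box and briefly toggles a particle emitter, then applies Scale to the player and restores unit scale after Duration.
; The construction script applies the Material variable to the mesh.
; An author note flags that rescaling sinks the character into the ground; the spent pickup is neither destroyed nor re-enabled.
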(event `self.HitBox.OnComponentBeginOverlap`
  (params (OtherActor :type "Actor Object Reference") (OtherComp :type "PrimitiveComponent Object Reference") (OtherBodyIndex :type Integer))
  (bind _particleemitter (`self.ParticleEmitter`))
  (bind _playerchar (`self.PlayerChar`))
  ;[1 1 1] Plocka upp powerup
  (bind _asmycharacter_c (cast `/Game/Blueprints/MyCharacter` OtherActor))
  (set `self.PlayerChar` _asmycharacter_c)
  (`ActorComponent.ToggleActive` _particleemitter)
  (`SceneComponent.SetHiddenInGame` (`self.SizePickupMesh`) true false)
  (`PrimitiveComponent.SetCollisionEnabled` (`self.HitBox`) "NoCollision")
  (`KismetSystemLibrary.Delay` 0.2)
  (`ActorComponent.ToggleActive` _particleemitter)
  ;[0.2575 0.6841 1] S?tter storleken, m?ste ses ?ver.. man landar i marken imellan?t.. eller ja, hela tiden.
  (`self.SetActorScale3D` _playerchar (`self.Scale`))
  (`KismetSystemLibrary.Delay` (`self.Duration`))
  (`self.SetActorScale3D` _playerchar (`KismetMathLibrary.MakeVector` 1.0 1.0 1.0)))

(fn `UserConstructionScript`
  (`PrimitiveComponent.SetMaterial` (`self.SizePickupMesh`) 0 (`self.Material`)))