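; Spotlight actor with a static mesh and a light whose brightness and tilt are set through its Intensity and Rotation variables.
; The construction script applies Intensity to the spotlight component, then passes Rotation to Turn.
; Turn sets the whole actor's pitch to the given degrees, taking yaw and roll from the mesh's current world rotation.
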(fn `Turn`
  (params (Degrees :type "Float (double-precision)"))
  (`self.SetActorRotation` (`KismetMathLibrary.MakeRot` Degrees (.yaw (`SceneComponent.K2_GetComponentRotation` (`self.StaticMesh1`))) (.roll (`SceneComponent.K2_GetComponentRotation` (`self.StaticMesh1`))))))

(fn `UserConstructionScript`
  (`LightComponent.SetBrightness` (`self.SpotLight1`) (`self.Intensity`))
  (`self.Turn` (`self.Rotation`)))